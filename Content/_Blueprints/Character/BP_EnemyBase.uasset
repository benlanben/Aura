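; Base enemy character Blueprint that handles spawn and death-dissolve visuals and attack facing.
; On BeginPlay, a timeline scales the mesh for a spawn effect.
; Dissolve events wait until shortly before the actor's lifespan ends, then timelines drive the Dissolve parameter on the supplied mesh and weapon dynamic materials, with the weapon starting later.
; UpdateFacingTarget feeds a location into the Motion Warping FacingTarget warp target.
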(event EventBeginPlay
  (bind _scaletrack (Timeline|SpawnTimeline Play)
    (:Update
      (Transformation|SetRelativeScale3D (Variables|Character|GetMesh) (Math|Vector|MakeVector _scaletrack _scaletrack _scaletrack)))))

(event Collision|EventActorBeginOverlap
  (params (OtherActor :type Actor%20Object%20Reference)))

(event EventTick
  (params (DeltaSeconds :type Float%20%28single-precision%29)))

(event EventStartMeshDissolveTimeline
  (params (DynamicMeshMaterialInstance :type Material%20Instance%20Dynamic%20Object%20Reference))
  (Utilities|FlowControl|Delay (- (Actor|GetLifeSpan) 3.0))
  (bind _meshdissolvetrack (Timeline|MeshDissolveTimeline Play)
    (:Update
      (Rendering|Material|SetScalarParameterValue DynamicMeshMaterialInstance "Dissolve" _meshdissolvetrack :!class /Script/Engine.MaterialInstanceDynamic))))

(event EventStartWeaponDissolveTimeline
  (params (DynamicWeaponMaterialInstance :type Material%20Instance%20Dynamic%20Object%20Reference))
  (Utilities|FlowControl|Delay (- (Actor|GetLifeSpan) 2.0))
  (bind _weapondissolvetrack (Timeline|WeaponDissolveTimeline Play)
    (:Update
      (Rendering|Material|SetScalarParameterValue DynamicWeaponMaterialInstance "Dissolve" _weapondissolvetrack :!class /Script/Engine.MaterialInstanceDynamic))))

(event EventUpdateFacingTarget
  (params (Target :type Vector%20%28by%20ref%29 :default "0, 0, 0"))
  (Class|MotionWarpingComponent|AddorUpdateWarpTargetfromLocation (Variables|Default|GetMotionWarping) "FacingTarget" Target))

(fn ConstructionScript)